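; BP_TaskIdentifier assigns itself a task number, derived from its own instance name.
; The construction script runs InitialiseTaskNum, which does nothing when ManualTaskNumOverride is set.
; Otherwise it chops the class name, less its '_C' suffix, from the display name and uses the numeric remainder as TaskNum, or 1 if empty.
; Reading the number from level data this way avoids additional save slots.
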(event Custom|InitialiseTaskNum
  (bind _self self)
  (bind _self_2 self)
  (bind _returnvalue (Utilities|GetClass _self_2))
  (bind _returnvalue_2 (Utilities|GetDisplayName _self))
  (bind _returnvalue_3 (Utilities|GetClassDisplayName _returnvalue))
  (bind _returnvalue_4 (Utilities|String|Len _returnvalue_3))
  (bind _returnvalue_5 (- _returnvalue_4 2))
  (bind _returnvalue_6 (Utilities|String|RightChop _returnvalue_2 _returnvalue_5))
  (if (not (Variables|BP_TaskIdentifierProperties|GetbManualTaskNumOverride?))
    ;[1 1 1] Set TaskNum in Accordance With Display Name (Prevents Use of Additional Save Slots - Required Data is Already Present in ULevel File)
    (if (Utilities|Enum|Equal(Enum) _returnvalue_6 "")
      (Variables|BP_TaskIdentifierProperties|SetTaskNum 1) ; If post-chop string is empty, \nmust be first TaskIdentifier\n(as it has no numerical suffix)
      (else
        (Variables|BP_TaskIdentifierProperties|SetTaskNum (Math|Conversions|ToInteger(Byte) _returnvalue_6)) ; Set TaskNum to value of \npost-chopped numerical suffix
      ))))

(fn ConstructionScript
  (CallFunction|InitialiseTaskNum))